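; Player controller for the main character that creates the HUD and handles pause, game over, level end and restart.
; BeginPlay binds the HUD to the pawn's health component and ranged weapon.
; GameOver plays death VFX and sound, swaps the HUD for a fade-out during time dilation, then resets GameInstance health.
; Pause keys open the menu; D-pad Up jumps from the easy challenge map to the challenge map once FirstWaveOver is set.
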(event Custom|EndLevel
  (Utilities|FlowControl|Delay 3.0)
  (bind _returnvalue (UserInterface|CreateWidget "/Game/UI/Menu/WB_GameOver.WB_GameOver_C"))
  (UserInterface|Viewport|AddtoViewport _returnvalue 0))

(event Custom|RestartLevel_
  (bind _returnvalue (Game|GetCurrentLevelName true))
  (Game|OpenLevel(byName) (Utilities|String|StringToName _returnvalue)))

(event Custom|GameOver
  (bind _returnvalue (Pawn|GetControlledPawn))
  (bind _time_dilation (Variables|Default|GetTime%20Dilation))
  (bind _mcdievfx (Variables|Default|GetMCDieVFX))
  (bind _returnvalue_2 (Transformation|GetActorLocation _returnvalue))
  ;[1 1 1] GameOver
  (Audio|PlaySoundatLocation "/Game/Audio/Game/Cue_GameOver.Cue_GameOver" _returnvalue_2 "0, 0, 0" 1.0 1.0 0.0 0 0 0 0)
  (Transformation|SetWorldLocation _mcdievfx _returnvalue_2 false false)
  (Components|Activation|SetActive _mcdievfx true false)
  (Utilities|Time|SetGlobalTimeDilation _time_dilation)
  (CallFunction|FadeOutEffect)
  (Utilities|FlowControl|Delay (* _time_dilation (Variables|Default|GetDuration)))
  (Utilities|Time|SetGlobalTimeDilation 1.0)
  (bind _asbp_game_instance (Utilities|Casting|CastToBP_GameInstance (Game|GetGameInstance)))
  (Default|ResetHealth _asbp_game_instance))

(event Custom|FadeOutEffect
  ;[1 1 1] GameOver
  (Widget|RemovefromParent (Variables|Default|GetPlayerHUD))
  (bind _returnvalue (UserInterface|CreateWidget "/Game/UI/Player/WB_GameOverFadeOut.WB_GameOverFadeOut_C"))
  (UserInterface|Viewport|AddtoViewport _returnvalue 0)
  (Default|PlayGameOverFadeOut _returnvalue))

(event EventBeginPlay
  (bind _asbp_mccharacter (Utilities|Casting|CastToBP_MCCharacter (Pawn|GetControlledPawn)))
  (Variables|Default|SetMCRef _asbp_mccharacter)
  (bind _asbp_weapon_mc (Utilities|Casting|CastToBP_Weapon_MC (Variables|/Script/Engine.ChildActorComponent|GetChildActor (Variables|/Game/Blueprint/MC/BP_MCCharacter.BP_MCCharacter_C|GetRangedWeapon _asbp_mccharacter))))
  (bind _returnvalue (UserInterface|CreateWidget "/Game/UI/Player/Player_HUD.Player_HUD_C" 0 (Actor|GetComponentbyClass (Pawn|GetControlledPawn) "/Game/Blueprint/Components/BPC_Health.BPC_Health_C") _asbp_weapon_mc))
  (bind _output_get (Variables|Default|SetPlayerHUD _returnvalue))
  (UserInterface|Viewport|AddtoViewport _output_get 0))

(event Input|GamepadEvents|GamepadDPadUp
  (params (Key :type Key%20Structure :default "None"))
  (:Pressed
    (if (Variables|Default|GetfirstWaveOver)
      (bind _returnvalue (Game|GetCurrentLevelName true))
      (if (Utilities|Enum|Equal(Enum) _returnvalue "TestMap_EasyChallenge")
        (Game|OpenLevel(byName) "TestMap_Challenge")))))

(event Input|KeyboardEvents|Escape
  (params (Key :type Key%20Structure :default "None"))
  (:Pressed
    (bind _returnvalue (UserInterface|CreateWidget "/Game/UI/Menu/WB_PauseMenu.WB_PauseMenu_C"))
    (UserInterface|Viewport|AddtoViewport _returnvalue 0)
    (Audio|PlaySound2D "/Game/Audio/UI/Cue_Pause.Cue_Pause" 1.0 1.0 0.0 0 0)))

(event Input|GamepadEvents|GamepadSpecialRight
  (params (Key :type Key%20Structure :default "None"))
  (:Pressed
    (bind _returnvalue (UserInterface|CreateWidget "/Game/UI/Menu/WB_PauseMenu.WB_PauseMenu_C"))
    (UserInterface|Viewport|AddtoViewport _returnvalue 0)
    (Audio|PlaySound2D "/Game/Audio/UI/Cue_Pause.Cue_Pause" 1.0 1.0 0.0 0 0)))

(event Input|KeyboardEvents|P
  (params (Key :type Key%20Structure :default "None"))
  (:Pressed
    (bind _returnvalue (UserInterface|CreateWidget "/Game/UI/Menu/WB_PauseMenu.WB_PauseMenu_C"))
    (UserInterface|Viewport|AddtoViewport _returnvalue 0)
    (Audio|PlaySound2D "/Game/Audio/UI/Cue_Pause.Cue_Pause" 1.0 1.0 0.0 0 0)))

(fn ConstructionScript)