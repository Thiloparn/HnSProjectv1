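; BP_Bullet is a data-driven projectile that damages actors and plays impact feedback.
; The construction script looks up its BulletName row in a data table for damage, speed and hit VFX, then sets ProjectileMovement speed.
; Sphere overlaps apply BP_BulletDamage only to actors implementing InterfaceToDamage, while blocking hits just play world impact feedback.
; Both spawn an effect and sound, then destroy the bullet; PlayVFX separately replays the explosion at the last overlap location.
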(event OnComponentHit(SphereCollision)
  (params (HitComponent :type Primitive%20Component%20Object%20Reference) (OtherActor :type Actor%20Object%20Reference) (OtherComp :type Primitive%20Component%20Object%20Reference) (NormalImpulse :type Vector :default "0, 0, 0") (Hit :type Hit%20Result%20Structure%20%28by%20ref%29))
  (Effects|SpawnEmitteratLocation (Variables|Default|GetHitWorldImpact) (.ImpactPoint (Collision|BreakHitResult Hit)))
  (Audio|PlaySoundatLocation "/Game/Audio/Enemies/Ranged/Cue_BulletImpactProp.Cue_BulletImpactProp" (Transformation|GetActorLocation) "0, 0, 0" 1.0 1.0 0.0 0 0 0 0)
  (Actor|DestroyActor))

(event OnComponentBeginOverlap(SphereCollision)
  (params (OverlappedComponent :type Primitive%20Component%20Object%20Reference) (OtherActor :type Actor%20Object%20Reference) (OtherComp :type Primitive%20Component%20Object%20Reference) (OtherBodyIndex :type Integer) (bFromSweep :type Boolean) (SweepResult :type Hit%20Result%20Structure%20%28by%20ref%29))
  (Variables|Default|SetHitActorLocation (.Location (Collision|BreakHitResult SweepResult)))
  (if (Utilities|DoesObjectImplementInterface OtherActor (Variables|Default|GetInterfaceToDamage))
    (Game|Damage|ApplyDamage OtherActor (Variables|Default|GetBulletDefaultDamage) 0 self "/Game/Blueprint/BP_BulletDamage.BP_BulletDamage_C")
    (Effects|SpawnEmitteratLocation (Variables|Default|GetExplosionEffect) (Variables|Default|GetHitActorLocation))
    (Audio|PlaySoundatLocation "/Game/Audio/Enemies/Ranged/Cue_BulletImpactPlayer.Cue_BulletImpactPlayer" (Transformation|GetActorLocation) "0, 0, 0" 1.0 1.0 0.0 0 0 0 0)
    (Actor|DestroyActor)))

(event Custom|PlayVFX
  (Effects|SpawnEmitteratLocation (Variables|Default|GetExplosionEffect) (Variables|Default|GetHitActorLocation)))

(fn ConstructionScript
  (bind _projectilemovement (Variables|Default|GetProjectileMovement))
  (bind _returnvalue (Utilities|GetDataTableRow (Variables|Default|GetDataTable) (Variables|Default|GetBulletName))
    (:then
      (Variables|Default|SetBulletDefaultDamage (.Damage (Utilities|Struct|BreakSBullet _returnvalue)))
      (Variables|Default|SetBulletSpeed (.Speed (Utilities|Struct|BreakSBullet _returnvalue)))
      (Variables|Default|SetExplosionEffect (.HitVFX (Utilities|Struct|BreakSBullet _returnvalue)))
      (Variables|Default|SetHitWorldImpact (.HitVFX (Utilities|Struct|BreakSBullet _returnvalue))))
    (:RowNotFound
      _))
  (Variables|/Script/Engine.ProjectileMovementComponent|SetInitialSpeed _projectilemovement (Variables|Default|GetBulletSpeed))
  (Variables|/Script/Engine.ProjectileMovementComponent|SetMaxSpeed _projectilemovement (Variables|Default|GetBulletSpeed)))