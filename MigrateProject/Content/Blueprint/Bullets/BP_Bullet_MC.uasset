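; Player character bullet projectile that damages enemies and plays impact effects, spawning with movement and collision disabled.
; Sphere overlaps treat static mesh components on damageable actors (InterfaceToDamage) as shields that block damage, while other components take BP_BulletDamage.
; The target's marked state selects explosion and enemy impact sound variants.
; Hits and other overlaps play prop impacts and destroy the bullet, except overlaps with BPI_MC actors, which are ignored.
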(event OnComponentHit(SphereCollision)
  (params (HitComponent :type Primitive%20Component%20Object%20Reference) (OtherActor :type Actor%20Object%20Reference) (OtherComp :type Primitive%20Component%20Object%20Reference) (NormalImpulse :type Vector :default "0, 0, 0") (Hit :type Hit%20Result%20Structure%20%28by%20ref%29))
  (Variables|Default|SetHitActorLocation (.Location (Collision|BreakHitResult Hit)))
  (CallFunction|PlayVFX)
  (CallFunction|PlayHitPropSound)
  (Actor|DestroyActor))

(event OnComponentBeginOverlap(SphereCollision)
  (params (OverlappedComponent :type Primitive%20Component%20Object%20Reference) (OtherActor :type Actor%20Object%20Reference) (OtherComp :type Primitive%20Component%20Object%20Reference) (OtherBodyIndex :type Integer) (bFromSweep :type Boolean) (SweepResult :type Hit%20Result%20Structure%20%28by%20ref%29))
  (bind (_bblockinghit _binitialoverlap _time _distance _location _impactpoint _normal _impactnormal _physmat _hitactor _hitcomponent) (Collision|BreakHitResult SweepResult))
  (Variables|Default|SetHit%20Actor OtherActor)
  (Variables|Default|SetHitActorLocation _location)
  (if (Utilities|DoesObjectImplementInterface OtherActor (Variables|Default|GetInterfaceToDamage))
    (bind _ismarked (Class|BPIEnemyBase|GetIsMarked(Message) (Variables|Default|GetHit%20Actor)))
    (Variables|Default|SetHitEnemyIsMarked _ismarked)
    (if (== (Utilities|GetClass _hitcomponent) "/Script/Engine.StaticMeshComponent")
      ;[1 1 1] Hit Shield
      (Effects|SpawnEmitteratLocation "/Game/VFX/MC/P_ImpactBulletShield.P_ImpactBulletShield" (Variables|Default|GetHitActorLocation))
      (CallFunction|PlayHitShield)
      (Actor|DestroyActor)
      (else
        ;[1 1 1] Hit Enemy
        (Game|Damage|ApplyDamage (Variables|Default|GetHit%20Actor) (Variables|Default|GetBulletMarkDamage) 0 self "/Game/Blueprint/BP_BulletDamage.BP_BulletDamage_C")
        (CallFunction|PlayVFX)
        (CallFunction|PlayHitEnemySound)
        (Actor|DestroyActor)))
    (elif (not (Utilities|DoesObjectImplementInterface OtherActor "/Game/Blueprint/MC/BPI_MC.BPI_MC_C"))
      (CallFunction|PlayVFX)
      (CallFunction|PlayHitPropSound)
      (Actor|DestroyActor))))

(event Custom|PlayHitPropSound
  ;[1 0.5649 0.8701] Audio
  (Audio|SpawnSoundatLocation "/Game/Audio/MC/Gun/Impacts/Cue_BulletImpactProp.Cue_BulletImpactProp" (Variables|Default|GetHitActorLocation) "0, 0, 0" 1.0 1.0 0.0 0 0))

(event Custom|PlayHitEnemySound
  ;[1 0.5649 0.8701] Audio
  (Audio|SpawnSoundatLocation (select (Variables|Default|GetHitEnemyIsMarked) "/Game/Audio/MC/Gun/Impacts/Cue_BulletImpactEnemy.Cue_BulletImpactEnemy" "/Game/Audio/MC/Gun/Impacts/Cue_ImpactEnemyWithoutMarks.Cue_ImpactEnemyWithoutMarks") (Variables|Default|GetHitActorLocation) "0, 0, 0" 1.0 1.0 0.0 0 0))

(event Custom|PlayHitShield
  ;[1 0.5649 0.8701] Audio
  (Audio|SpawnSoundatLocation "/Game/Audio/MC/Gun/Impacts/Cue_ImpactShield.Cue_ImpactShield" (Variables|Default|GetHitActorLocation) "0, 0, 0" 1.0 1.0 0.0 0 0))

(event EventBeginPlay
  (Components|Activation|SetActive (Variables|Default|GetProjectileMovement) false false))

(event EventPlayVFX
  (Effects|SpawnEmitteratLocation (select (Variables|Default|GetHitEnemyIsMarked) (Variables|Default|GetExplosionEffect) (Variables|VFX|GetExplosionEffectWithoutMarks)) (Variables|Default|GetHitActorLocation)))

(fn ConstructionScript
  (|CallParentFunction)
  (Collision|SetCollisionEnabled (Variables|Default|GetSphereCollision) "NoCollision"))