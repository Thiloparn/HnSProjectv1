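; BP_Door is a level entrance or exit door that animates open and closed and handles map transitions.
; Non-exit doors close on BeginPlay under a transition widget.
; OpenDoor waits, plays sound, then a timeline swings both leaves, fades in the floor and saves player health to the GameInstance.
; Box overlap by a BPI_MC actor shows victory screens or plays an exit transition, whose end callback loads NextLevel.
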(event OnComponentBeginOverlap(Box)
  (params (OverlappedComponent :type Primitive%20Component%20Object%20Reference) (OtherActor :type Actor%20Object%20Reference) (OtherComp :type Primitive%20Component%20Object%20Reference) (OtherBodyIndex :type Integer) (bFromSweep :type Boolean) (SweepResult :type Hit%20Result%20Structure%20%28by%20ref%29))
  ;[1 1 1] Overlap
  (if (Utilities|DoesObjectImplementInterface OtherActor "/Game/Blueprint/MC/BPI_MC.BPI_MC_C")
    (if (== (Variables|Default|GetNextLevel) "Victory")
      ;[1 1 1] Victory
      (Audio|PlaySound2D "/Game/Audio/Game/Cue_Victory.Cue_Victory" 1.0 1.0 0.0 0 0)
      (bind _returnvalue (UserInterface|CreateWidget "/Game/UI/Player/WB_VictoryFadeOut.WB_VictoryFadeOut_C"))
      (UserInterface|Viewport|AddtoViewport _returnvalue 0)
      (Default|PlayVictoryFadeOut _returnvalue)
      (Utilities|FlowControl|Delay 1.8)
      (bind _returnvalue_2 (UserInterface|CreateWidget "/Game/UI/Menu/WB_Victory.WB_Victory_C"))
      (UserInterface|Viewport|AddtoViewport _returnvalue_2 0)
      (else
        (bind _returnvalue_3 (UserInterface|CreateWidget "/Game/UI/Menu/WB_MapTransition.WB_MapTransition_C" 0 true))
        (UserInterface|Viewport|AddtoViewport _returnvalue_3 0)
        (EventDispatchers|AssignOnAnimEnd _returnvalue_3 (delegate Custom|OnAnimEnd_Event))))))

(event Custom|OpenDoor
  ;[1 1 1] Open
  (Utilities|FlowControl|Delay (Variables|Default|GetOpeningDelay))
  (Components|Timeline|SetPlayRate (Variables|Default|GetTimeline) (/ 1.0 (Variables|Default|GetAnimDuration)))
  (CallFunction|PlayDoorSound)
  (bind _newtrack_0 (Timeline|Timeline Play)
    (:Update
      (Transformation|SetRelativeRotation (Variables|Default|GetDoorLeft) (Math|Rotator|MakeRotator 0.0 0.0 (Math|Float|Lerp 0.0 9e+01 _newtrack_0)) false false)
      (Transformation|SetRelativeRotation (Variables|Default|GetDoorRight) (Math|Rotator|MakeRotator 0.0 0.0 (* (Math|Float|Lerp 0.0 9e+01 _newtrack_0) -1.0)) false false)
      (Rendering|Material|SetScalarParameterValueonMaterials (Variables|Default|GetFloor) "Opacity" _newtrack_0))
    (:Finished
      (Variables|Default|SetbIsOpen true)
      (bind _asbp_mccharacter (Utilities|Casting|CastToBP_MCCharacter (Game|Player|GetPlayerPawn 0)))
      (bind _asbp_game_instance (Utilities|Casting|CastToBP_GameInstance (Game|GetGameInstance)))
      (Variables|/Game/Blueprint/General/BP_GameInstance.BP_GameInstance_C|SetPlayerHealth _asbp_game_instance (Variables|/Game/Blueprint/Components/BPC_Health.BPC_Health_C|GetHealth (Variables|/Game/Blueprint/MC/BP_MCCharacter.BP_MCCharacter_C|GetBPC_Health _asbp_mccharacter))))))

(event Custom|Close
  ;[1 1 1] Close
  (Components|Timeline|SetPlayRate (Variables|Default|GetTimeline) (/ 1.0 (Variables|Default|GetAnimDuration)))
  (bind _newtrack_0 (Timeline|Timeline_0 PlayFromStart)
    (:Update
      (Transformation|SetRelativeRotation (Variables|Default|GetDoorLeft) (Math|Rotator|MakeRotator 0.0 0.0 (Math|Float|Lerp -6e+01 0.0 _newtrack_0)) false false))
    (:Finished
      (Variables|Default|SetbIsOpen false))))

(event Custom|OnAnimEnd_Event
  ;[1 1 1] Overlap
  (Game|OpenLevel(byName) (Variables|Default|GetNextLevel)))

(event Custom|PlayDoorSound
  (bind _audiocomponent (Variables|Default|GetAudioComponent))
  (if (Variables|Default|GetbIsOpen)
    (Audio|Components|Audio|SetSound _audiocomponent "/Game/Audio/Environment/Cue_CloseDoor.Cue_CloseDoor")
    (Audio|Components|Audio|Play _audiocomponent 0.0)
    (else
      (Audio|Components|Audio|SetSound _audiocomponent "/Game/Audio/Environment/Cue_OpenDoor.Cue_OpenDoor")
      (Audio|Components|Audio|Play _audiocomponent 0.0))))

(event EventBeginPlay
  ;[1 1 1] Begin Play
  (Rendering|Material|SetScalarParameterValueonMaterials (Variables|Default|GetFloor) "Opacity" 0.0)
  (if (not (Variables|Default|GetbIsExit))
    (CallFunction|Close)
    (bind _returnvalue (UserInterface|CreateWidget "/Game/UI/Menu/WB_MapTransition.WB_MapTransition_C"))
    (UserInterface|Viewport|AddtoViewport _returnvalue 0)))

(fn ConstructionScript)