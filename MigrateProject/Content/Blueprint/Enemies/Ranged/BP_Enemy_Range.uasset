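; BP_Enemy_Range is a ranged enemy that extends a parent enemy class and fires bullets at the player.
; Its Attack override plays the pistol reload montage and fires only when the montage completes.
; It then calls the parent Attack, rotates BulletSpawn toward player pawn 0, spawns BP_Bullet with itself as Instigator and activates the muzzle VFX.
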(event EventAttack
  (bind _bulletspawn (Variables|Default|GetBulletSpawn))
  (Animation|Montage|PlayMontage (Variables|Character|GetMesh) "/Game/Animations/Animations/Custom/AM_PistolReload.AM_PistolReload"
    (:OnCompleted
      (|CallParentFunction)
      (Transformation|SetWorldRotation _bulletspawn (Math|Rotator|FindLookatRotation (Transformation|GetWorldLocation _bulletspawn) (Transformation|GetActorLocation (Game|Player|GetPlayerPawn 0))) false false)
      (Game|SpawnActorfromClass "/Game/Blueprint/Bullets/BP_Bullet.BP_Bullet_C" (Transformation|GetWorldTransform (Variables|Default|GetBulletSpawn)) "Undefined" "MultiplyWithRoot" 0 "EnemyBullet" self)
      (Components|Activation|Activate (Variables|Default|GetMuzzleVFX) false))))

(fn ConstructionScript
  (|CallParentFunction))