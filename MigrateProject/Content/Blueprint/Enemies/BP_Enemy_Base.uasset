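; Base enemy character that rises from the ground on spawn, feeds behavior tree blackboard flags for player detection and stagger, and handles attack montages and death.
; A looping timer detects the player by distance and line-of-sight trace.
; Melee hits add marks and stagger without damaging health; bullets only damage marked, unshielded enemies by consuming marks, with overlay-material flashes.
; Also provides a timed shield and a radial mark explosion.
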(event Custom|Attack
  ;[1 1 1] Attack
  (Animation|Montage|PlayMontage (Variables|Character|GetMesh) (Variables|TypeSpecific|GetAttackMontage)
    (:OnCompleted
      _)
    (:OnInterrupted
      _))
  (Default|CallOnAttackEnd))

(event Custom|Death
  (params (Actor :type Actor%20Object%20Reference))
  ;[1 1 1] Begin Play
  (CallFunction|ChangetoDeathCollision)
  (Components|Activation|Activate (Variables|Default|GetDeathVFX) false)
  (Actor|SetLifeSpan (Variables|Death|GetLifespan))
  (Audio|PlaySoundatLocation (Variables|Audio|GetDeathSFX) (Transformation|GetActorLocation) "0, 0, 0" 1.0 1.0 0.0 0 0 0 0))

(event Custom|DamagedOverlayColor
  (params (bIsMelee :type Boolean) (NumMarks :type Integer))
  (bind _overlaymaterial (Variables|Default|GetOverlayMaterial))
  ;[1 1 1] Damaged Colors
  (Rendering|Material|SetVectorParameterValue _overlaymaterial "Color" (Math|Color|SelectColor "(R=1.000000,G=1.000000,B=1.000000,A=1.000000)" (Utilities|Select :Index (Math|Integer|Min(Integer) NumMarks 3) :Option%200 "(R=1.000000,G=0.000000,B=0.542838,A=1.000000)" :Option%201 "(R=1.000000,G=0.831373,B=0.000000,A=1.000000)" :Option%202 "(R=1.000000,G=0.168627,B=0.000000,A=1.000000)" :Option%203 "(R=0.741176,G=0.007843,B=0.000000,A=1.000000)") bIsMelee) :!class /Script/Engine.MaterialInstanceDynamic)
  (Rendering|Material|SetScalarParameterValue _overlaymaterial "Opacity" 0.1 :!class /Script/Engine.MaterialInstanceDynamic)
  (Utilities|FlowControl|Delay 0.3)
  (Rendering|Material|SetScalarParameterValue _overlaymaterial "Opacity" 0.0 :!class /Script/Engine.MaterialInstanceDynamic))

(event Custom|SetShield
  (bind _shield (Variables|Default|GetShield))
  (bind _shield_2 (Variables|Default|GetShield))
  ;[1 1 1] Shield
  (Variables|Default|SetbHasShield true)
  (Rendering|SetVisibility _shield_2 true false)
  (Collision|SetCollisionEnabled _shield_2 "QueryAndPhysics")
  (Audio|Components|Audio|Play (Variables|Default|GetAudio) 0.0)
  (Utilities|FlowControl|RetriggerableDelay 4.0)
  (Audio|Components|Audio|Stop (Variables|Default|GetAudio))
  (Variables|Default|SetbHasShield false)
  (Rendering|SetVisibility _shield false false)
  (Collision|SetCollisionEnabled _shield "NoCollision"))

(event Custom|SpawnAnim
  (bind _returnvalue (Transformation|GetActorLocation))
  (bind _capsulecomponent (Variables|Collision|GetCapsuleComponent))
  (bind _mesh (Variables|Character|GetMesh))
  (bind _capsulehalfheight (Variables|/Script/Engine.CapsuleComponent|GetCapsuleHalfHeight _capsulecomponent))
  (bind _returnvalue_2 (- _capsulehalfheight 1e+01))
  (bind _returnvalue_3 (- (.z _returnvalue) _returnvalue_2))
  (bind _returnvalue_4 (Math|Vector|MakeVector (.x _returnvalue) (.y _returnvalue) _returnvalue_3))
  ;[1 1 1] Spawn
  (bind _output_get (Variables|SpawnAnim|SetMeshZLocation (.z (Variables|/Script/Engine.SceneComponent|GetRelativeLocation _mesh))))
  (bind _output_get_2 (Variables|SpawnAnim|SetMeshZHiddenLocation (- _output_get (* (.SphereRadius (Math|BoxSphereBounds|BreakBoxSphereBounds (StaticMesh|GetBounds (Components|SkeletalMesh|GetSkeletalMeshAsset _mesh)))) 2.0))))
  (Transformation|SetRelativeLocation (Variables|Character|GetMesh) (Math|Vector|MakeVector 0.0 0.0 _output_get_2) false false)
  (bind _returnvalue_5 (Effects|SpawnEmitteratLocation "/Game/VFX/Enemy/P_Enemy_SpawnOpen.P_Enemy_SpawnOpen" _returnvalue_4 "90.000000,0.000000,0.000000" (Variables|/Script/Engine.SceneComponent|GetRelativeScale3D (Variables|Character|GetMesh))))
  (Utilities|FlowControl|Delay (Variables|SpawnAnim|GetSpawnDelay))
  (Components|Timeline|SetPlayRate (Variables|Default|GetTL_Spawn) (/ 1.0 (- (Variables|SpawnAnim|GetSpawnDuration) 0.5)))
  (bind _newtrack_0 (Timeline|TL_Spawn PlayFromStart)
    (:Update
      (Transformation|SetRelativeLocation (Variables|Character|GetMesh) (Math|Vector|MakeVector 0.0 0.0 (Math|Float|Lerp (Variables|SpawnAnim|GetMeshZHiddenLocation) (Variables|SpawnAnim|GetMeshZLocation) _newtrack_0)) false false))
    (:Finished
      (Components|Activation|Deactivate _returnvalue_5)
      (Effects|SpawnEmitteratLocation "/Game/VFX/Enemy/P_Enemy_SpawnClose.P_Enemy_SpawnClose" _returnvalue_4 "90.000000,0.000000,0.000000" (Variables|/Script/Engine.SceneComponent|GetRelativeScale3D (Variables|Character|GetMesh))))))

(event Custom|PlayerDetectionTimer
  ;[1 1 1] PlayerDetection
  (Utilities|Time|SetTimerbyEvent (delegate Custom|PlayerDetection) 0.1 true))

(event Custom|PlayerDetection
  (bind _returnvalue (Pawn|GetController))
  (bind _returnvalue_2 (AI|GetBlackboard _returnvalue))
  ;[1 1 1] PlayerDetection
  (if (not (Variables|Default|GetbIsPlayerDetected))
    (if (and (<= (Math|Vector|Distance2D(Vector) (Transformation|GetActorLocation) (Transformation|GetActorLocation (Game|GetPlayerCharacter 0))) (Variables|Default|GetDetectionDistance)) (Utilities|IsValid _returnvalue_2))
      (bind _returnvalue_3 (Collision|LineTraceByChannel (Transformation|GetActorLocation) (Transformation|GetActorLocation (Game|GetPlayerCharacter 0)) "TraceTypeQuery1" false 0 "None"))
      (if (not _returnvalue_3)
        (Variables|Default|SetbIsPlayerDetected true)
        (AI|Components|Blackboard|SetValueasBool _returnvalue_2 (Utilities|Name|MakeLiteralName "bIsPlayerDetected") true)))))

(event Game|Damage|EventAnyDamage
  (params (Damage :type Float%20%28single-precision%29) (DamageType :type Damage%20Type%20Object%20Reference) (InstigatedBy :type Controller%20Object%20Reference) (DamageCauser :type Actor%20Object%20Reference))
  (bind _bpc_marks (Variables|Default|GetBPC_Marks))
  ;[1 1 1] Any Damage
  (if (Class|GameplayStatics|ObjectIsA DamageType "/Game/Blueprint/BP_MeleeDamage.BP_MeleeDamage_C")
    (Default|AddMark (Variables|Default|GetBPC_Marks))
    (Class|NavMovementComponent|StopActiveMovement (Variables|Character|GetCharacterMovement))
    (if (Variables|HitReceiving|GetbGetPushed)
      (Character|LaunchCharacter (* (Transformation|GetActorForwardVector DamageCauser) (Variables|HitReceiving|GetPushForce)) false false))
    (CallFunction|Stagger)
    (CallFunction|DamagedOverlayColor true)
    (elif (Class|GameplayStatics|ObjectIsA DamageType "/Game/Blueprint/BP_BulletDamage.BP_BulletDamage_C")
      (if (Variables|/Game/Blueprint/Components/BPC_Marks.BPC_Marks_C|GetbIsMarked _bpc_marks)
        (if (not (Variables|Default|GetbHasShield))
          (CallFunction|Stagger)
          (bind (_finaldamage _numconsumedmarks) (Default|ConsumeMark _bpc_marks Damage))
          (CallFunction|DamagedOverlayColor false _numconsumedmarks)
          (Default|DecreaseHealth (Variables|Default|GetBPC_Health) _finaldamage))))))

(event EventBeginPlay
  ;[1 1 1] Begin Play
  (Components|Timeline|SetPlayRate (Variables|Default|GetTL_IncreaseSphere) 2.5)
  (bind _returnvalue (UserInterface|CreateWidget "/Game/UI/Enemies/WB_HealthNPostureBar_v3.WB_HealthNPostureBar_v3_C" 0 (Variables|Default|GetBPC_Health) 0))
  (UserInterface|SetWidget (Variables|Default|GetHnPWidget) _returnvalue)
  (Variables|/Game/Blueprint/Components/BPC_Marks.BPC_Marks_C|SetHealthNPostureWB (Variables|Default|GetBPC_Marks) _returnvalue)
  (EventDispatchers|BindEventtoOnDeath (Variables|Default|GetBPC_Health) (delegate Custom|Death))
  (CallFunction|SpawnAnim)
  (CallFunction|PlayerDetectionTimer))

(event EventMarkExplosion
  (bind _returnvalue (Transformation|GetActorLocation))
  (bind _returnvalue_2 (Transformation|GetActorLocation))
  ;[1 1 1] MarkExplosion
  (CallFunction|Stagger)
  (bind (_outhits _returnvalue_3) (Collision|MultiSphereTraceForObjects _returnvalue_2 _returnvalue_2 (Variables|Default|GetMarkExplosionRadius) (Utilities|Array|MakeArray "ObjectTypeQuery3") false 0 "None"))
  (if _returnvalue_3
    (for _array_element _outhits
      (if (Utilities|DoesObjectImplementInterface (.HitActor (Collision|BreakHitResult _array_element)) "/Game/Blueprint/MC/BPI_MC.BPI_MC_C")
        (Class|BPIMC|HitbyExplosion(Message) (.HitActor (Collision|BreakHitResult _array_element)) (Transformation|GetActorLocation) "0, 0, 0")
        (Game|Damage|ApplyDamage (.HitActor (Collision|BreakHitResult _array_element)) 1e+01 0 self "/Game/Blueprint/BP_BulletDamage.BP_BulletDamage_C")
        (else
          (bind _asbp_enemy_base (Utilities|Casting|CastToBP_Enemy_Base (.HitActor (Collision|BreakHitResult _array_element))))
          (CallFunction|Stagger _asbp_enemy_base))))
    (bind _alpha (Timeline|TL_IncreaseSphere PlayFromStart)
      (:Update
        (Rendering|Debug|DrawDebugSphere (Math|Vector|MakeVector (.x _returnvalue) (.y _returnvalue) (- (.z _returnvalue) 6e+01)) (* _alpha (Variables|Default|GetMarkExplosionRadius)) 24 "(R=1.000000,G=0.000000,B=0.000000,A=1.000000)" 0.0)))
    (else
      (Timeline|TL_IncreaseSphere PlayFromStart))))

(fn ConstructionScript
  (bind _returnvalue (Rendering|Material|CreateDynamicMaterialInstance "/Game/Materials/M_DamagedOverlay.M_DamagedOverlay" "None" "None" :!class /Script/Engine.KismetMaterialLibrary))
  (bind _output_get (Variables|Default|SetOverlayMaterial _returnvalue))
  (Rendering|Material|SetOverlayMaterial (Variables|Character|GetMesh) _output_get :!class /Script/Engine.MeshComponent))

(fn ChangetoDeathCollision
  (bind _capsulecomponent (Variables|Collision|GetCapsuleComponent))
  (Collision|SetCollisionEnabled _capsulecomponent "NoCollision")
  (Collision|SetCollisionObjectType _capsulecomponent "ECC_WorldStatic")
  (Collision|SetCollisionObjectType (Variables|Character|GetMesh) "ECC_WorldStatic"))

(fn Stagger
  (bind _returnvalue (AI|GetBlackboard 0))
  (bind _returnvalue_2 (Utilities|Name|MakeLiteralName "bIsStaggered"))
  (if (Variables|Default|GetbShouldHitReact)
    (Animation|Montage|MontagePlay (Components|SkeletalMesh|GetAnimInstance (Variables|Character|GetMesh)) "/Game/Animations/Animations/Custom/AM_HitReaction.AM_HitReaction" 1.0 "MontageLength" 0.0 (Variables|HitReceiving|GetbCanBeStaggered)))
  (if (Variables|HitReceiving|GetbCanBeStaggered)
    (Components|Movement|StopMovementImmediately (Variables|Character|GetCharacterMovement))
    (AI|Components|Blackboard|SetValueasBool _returnvalue _returnvalue_2 false)
    (AI|Components|Blackboard|SetValueasBool _returnvalue _returnvalue_2 true)))

(fn GetControllerData
  (return (Variables|GeneralData|GetBehaviorTree) (Variables|SpawnAnim|GetSpawnDuration)))

(fn GetIsMarked
  (return (Variables|/Game/Blueprint/Components/BPC_Marks.BPC_Marks_C|GetbIsMarked (Variables|Default|GetBPC_Marks))))

(fn GetStrafeDistance
  (return (Variables|TypeSpecific|GetStrafeDistance)))

(fn SetMovementSpeed
  (params (MovementEnum :type E_MovementSpeed%20Enum :default "NewEnumerator0"))
  (bind _output_get (Variables|/Script/Engine.CharacterMovementComponent|SetMaxWalkSpeed (Variables|Character|GetCharacterMovement) (Utilities|Select :Index MovementEnum :NewEnumerator0 (Variables|Movement|GetRunning%20Speed) :NewEnumerator1 (Variables|Movement|GetStrafing%20Speed))))
  (return _output_get))