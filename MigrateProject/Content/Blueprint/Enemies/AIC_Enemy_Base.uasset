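; Base AI controller for enemies that starts their behavior tree when it possesses a pawn.
; It asks the pawn through message calls for its behavior tree, spawn duration and strafe distance, so each enemy supplies its own setup.
; After waiting out the spawn duration, it runs the tree and writes the strafe distance and the player character into the Blackboard.
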(event EventPossess
  (params (PossessedPawn :type Pawn%20Object%20Reference))
  (bind _blackboard (Variables|Default|GetBlackboard))
  (Utilities|FlowControl|DelayUntilNextTick)
  (bind (_behaviortree _spawnduration) (Class|BPIEnemyBase|GetControllerData(Message) PossessedPawn))
  (Utilities|IsValid _behaviortree
    (:Is%20Valid
      (Utilities|FlowControl|Delay _spawnduration)
      (AI|RunBehaviorTree _behaviortree)
      (bind _strafedistance (Class|BPIEnemyBase|GetStrafeDistance(Message) PossessedPawn))
      (AI|Components|Blackboard|SetValueasFloat _blackboard (Utilities|Name|MakeLiteralName "StrafeDistance") _strafedistance)
      (AI|Components|Blackboard|SetValueasObject _blackboard (Utilities|Name|MakeLiteralName "MC") (Game|GetPlayerCharacter 0)))))

(fn ConstructionScript)