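; BPC_AttackToken is a component that tracks a pool of attack tokens for each attacker tag, gating attacks by availability.
; TakeToken deducts the requested amount from the tag's count in the AttackTokenCount map, failing if the tag is missing or short.
; ReturnToken adds the amount back without an upper limit and always reports success.
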(fn TakeToken
  (params (Amount :type Integer) (AttackerTag :type Gameplay%20Tag%20Structure))
  (bind _attacktokencount (Variables|Default|GetAttackTokenCount))
  (bind (_value _returnvalue) (Utilities|Map|Find _attacktokencount AttackerTag))
  (if _returnvalue
    (if (<= Amount _value)
      (Utilities|Map|Add (Variables|Default|GetAttackTokenCount) AttackerTag (- _value Amount))
      (return true)
      (else
        _)))
  (return false))

(fn ReturnToken
  (params (Amount :type Integer) (AttackerTag :type Gameplay%20Tag%20Structure))
  (Utilities|Map|Add (Variables|Default|GetAttackTokenCount) AttackerTag (+ Amount (.Value (Utilities|Map|Find (Variables|Default|GetAttackTokenCount) AttackerTag))))
  (return true))