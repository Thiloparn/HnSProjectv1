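; Biggy enemy Blueprint whose attack is a telegraphed straight-line charge toward the player's position, locked in when the attack starts.
; After anticipation, a duration-scaled Timeline sweeps it along a flattened path while its capsule overlaps pawns, damaging and notifying the first BPI_MC actor hit.
; The charge drives AnimBP flags, VFX and sounds, then plays a tired montage before signalling attack end.
; Melee damage disables hit reactions.
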(event OnComponentBeginOverlap(CapsuleComponent)
  (params (OverlappedComponent :type Primitive%20Component%20Object%20Reference) (OtherActor :type Actor%20Object%20Reference) (OtherComp :type Primitive%20Component%20Object%20Reference) (OtherBodyIndex :type Integer) (bFromSweep :type Boolean) (SweepResult :type Hit%20Result%20Structure%20%28by%20ref%29))
  (bind _returnvalue (Transformation|GetActorLocation))
  (if (and (Variables|/Game/Blueprint/Enemies/Biggy/ABP_Enemy_Biggy.ABP_Enemy_Biggy_C|GetisCharging (Variables|Default|GetABP%20Enemy%20Biggy)) (not (Variables|Default|GetbHasHit)))
    (if (Utilities|DoesObjectImplementInterface OtherActor "/Game/Blueprint/MC/BPI_MC.BPI_MC_C")
      (Variables|Default|SetbHasHit true)
      (Game|Damage|ApplyDamage OtherActor (Variables|Default|GetChargeDamage) 0 self "/Game/Blueprint/BP_BulletDamage.BP_BulletDamage_C")
      (Class|BPIMC|HitbyExplosion(Message) OtherActor _returnvalue (Variables|Default|GetChargeTargetLocation))
      (Audio|PlaySoundatLocation "/Game/Audio/Enemies/Biggy/Cue_BiggyHitsPlayer.Cue_BiggyHitsPlayer" _returnvalue "0, 0, 0" 1.0 1.0 0.0 0 0 0 0))))

(event Custom|ChargeAttack
  (bind _returnvalue (Transformation|GetActorLocation))
  (bind _returnvalue_2 (Game|Player|GetPlayerPawn 0))
  (bind _abp_enemy_biggy (Variables|Default|GetABP%20Enemy%20Biggy))
  (bind _returnvalue_3 (Transformation|GetActorLocation _returnvalue_2))
  (bind _returnvalue_4 (Math|Vector|GetUnitDirection(Vector) _returnvalue _returnvalue_3))
  (Audio|PlaySoundatLocation "/Game/Audio/Enemies/Biggy/Cue_BiggyChargingDash.Cue_BiggyChargingDash" (Transformation|GetActorLocation) "0, 0, 0" 1.0 1.0 0.0 0 0 0 0)
  (Components|Timeline|SetPlayRate (Variables|Default|GetTimeline) (/ 1.0 (Variables|Default|GetChargeDuration)))
  (bind _output_get (Variables|Default|SetChargeInitialLocation _returnvalue))
  (Variables|Default|SetChargeTargetLocation (+ _output_get (* (Math|Vector|MakeVector (.x _returnvalue_4) (.y _returnvalue_4) 0.0) (Variables|Default|GetChargeDistance))))
  (Variables|/Game/Blueprint/Enemies/Biggy/ABP_Enemy_Biggy.ABP_Enemy_Biggy_C|SetisAnticipating (Variables|Default|GetABP%20Enemy%20Biggy) true)
  (Utilities|FlowControl|Delay (Variables|Default|GetAnticipationDuration))
  (Variables|/Game/Blueprint/Enemies/Biggy/ABP_Enemy_Biggy.ABP_Enemy_Biggy_C|SetisAnticipating _abp_enemy_biggy false)
  (Variables|/Game/Blueprint/Enemies/Biggy/ABP_Enemy_Biggy.ABP_Enemy_Biggy_C|SetisCharging _abp_enemy_biggy true)
  (Variables|Default|SetbHasHit false)
  (Collision|SetCollisionResponsetoChannel (Variables|Default|GetCapsuleComponent) "ECC_Pawn" "ECR_Overlap")
  (Components|Activation|Activate (Variables|Default|GetTrailVFX) false)
  (Audio|PlaySoundatLocation "/Game/Audio/Enemies/Biggy/Cue_BiggyDashingForward.Cue_BiggyDashingForward" (Transformation|GetActorLocation) "0, 0, 0" 1.0 1.0 0.0 0 0 0 0)
  (bind _newtrack_0 (Timeline|Timeline PlayFromStart)
    (:Update
      (Transformation|SetActorLocation (Math|Vector|Lerp(Vector) (Variables|Default|GetChargeInitialLocation) (Variables|Default|GetChargeTargetLocation) _newtrack_0) true false))
    (:Finished
      (Variables|/Game/Blueprint/Enemies/Biggy/ABP_Enemy_Biggy.ABP_Enemy_Biggy_C|SetisCharging (Variables|Default|GetABP%20Enemy%20Biggy) false)
      (Collision|SetCollisionResponsetoChannel (Variables|Default|GetCapsuleComponent) "ECC_Pawn" "ECR_Block")
      (Components|Activation|Deactivate (Variables|Default|GetTrailVFX))
      (Animation|Montage|PlayMontage (Variables|Character|GetMesh) "/Game/Animations/Animations/Custom/AM_BiggyTired.AM_BiggyTired"
        (:OnCompleted
          _)
        (:OnInterrupted
          _))
      (Default|CallOnAttackEnd))))

(event EventBeginPlay
  (|CallParentFunction)
  (bind _asabp_enemy_biggy (Utilities|Casting|CastToABP_Enemy_Biggy (Components|SkeletalMesh|GetAnimInstance (Variables|Character|GetMesh))))
  (Variables|Default|SetABP%20Enemy%20Biggy _asabp_enemy_biggy))

(event Game|Damage|EventAnyDamage
  (params (Damage :type Float%20%28single-precision%29) (DamageType :type Damage%20Type%20Object%20Reference) (InstigatedBy :type Controller%20Object%20Reference) (DamageCauser :type Actor%20Object%20Reference))
  (Variables|Default|SetbShouldHitReact (not (Class|GameplayStatics|ObjectIsA DamageType "/Game/Blueprint/BP_MeleeDamage.BP_MeleeDamage_C")))
  (|CallParentFunction Damage DamageType InstigatedBy DamageCauser))

(fn ConstructionScript
  (|CallParentFunction))