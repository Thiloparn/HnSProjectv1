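; Melee enemy Blueprint that detects weapon hits on the player character and applies damage.
; DamageDetection sphere-traces for Pawns at the right-hand weapon socket and, on hitting BP_MCCharacter, applies damage using BP_BulletDamage with impact VFX and a sound.
; A HasHit flag limits each attack to one hit until ResetHasHit clears it.
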(fn ConstructionScript
  (|CallParentFunction))

(fn DamageDetection
  (bind _mesh (Variables|Character|GetMesh))
  (bind _returnvalue (Transformation|GetSocketLocation _mesh "weapon_r_socket"))
  (if (Variables|Default|GetbHasHit)
    _
    (else
      (bind (_outhit _returnvalue_2) (Collision|SphereTraceForObjects _returnvalue _returnvalue (Variables|MeleeEnemyAttack|GetHit%20Sphere%20Radius) (Utilities|Array|MakeArray "ObjectTypeQuery3") false 0 "None"))
      (if _returnvalue_2
        (if (Class|GameplayStatics|ObjectIsA (.HitActor (Collision|BreakHitResult _outhit)) "/Game/Blueprint/MC/BP_MCCharacter.BP_MCCharacter_C")
          (Variables|Default|SetbHasHit true)
          (Game|Damage|ApplyDamage (.HitActor (Collision|BreakHitResult _outhit)) (Variables|MeleeEnemyAttack|GetDamage) 0 self "/Game/Blueprint/BP_BulletDamage.BP_BulletDamage_C")
          (Effects|SpawnEmitteratLocation (Variables|Default|GetImpactVFX) (.ImpactPoint (Collision|BreakHitResult _outhit)))
          (Audio|PlaySoundatLocation (Variables|Audio|GetHitPlayerSFX) (Transformation|GetActorLocation) "0, 0, 0" 1.0 1.0 0.0 0 0 0 0)
          (return true)
          (else
            _)))))
  (return false))

(fn ResetHasHit
  (bind _output_get (Variables|Default|SetbHasHit false))
  (return _output_get))