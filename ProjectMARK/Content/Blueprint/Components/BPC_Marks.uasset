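; Component that tracks stacking marks on its owner, which are consumed for bonus damage based on summed per-stack multipliers.
; AddMark refreshes the timer and stops stacking at the cap or once the player's bullet damage would be lethal.
; Retriggerable delays expire marks one by one, with an advance warning animation.
; The health/posture widget displays marks and supplies current health; mark sound helpers sit on unconnected nodes.
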(event Custom|ResetMarks
  (Variables|DontEdit|SetMarks 0)
  (Default|ResetMarksUI (Variables|DontEdit|GetHealthNPostureWB))
  (Variables|DontEdit|SetbIsMarked false))

(event Custom|MarkTimer
  (Default|UpdateExpiredAnim (Variables|DontEdit|GetHealthNPostureWB) true)
  (Utilities|FlowControl|Sequence
    (:then_0
      (Utilities|FlowControl|RetriggerableDelay (Variables|Edit|GetMarkDuration))
      (if (> (Variables|DontEdit|GetMarks) 0)
        (Variables|DontEdit|SetMarks (Math|Integer|Max(Integer) (- (Variables|DontEdit|GetMarks) 1)))
        (Default|ExpireMarkUI (Variables|DontEdit|GetHealthNPostureWB))
        (bind _output_get (Variables|DontEdit|SetbIsMarked (> (Variables|DontEdit|GetMarks) 0)))
        (if _output_get
          (CallFunction|MarkTimer)
          (else
            (CallFunction|ResetMarks)))))
    (:then_1
      (Utilities|FlowControl|RetriggerableDelay (- (Variables|Edit|GetMarkDuration) (Variables|Edit|GetExpireAnimDuration)))
      (if (> (Variables|DontEdit|GetMarks) 0)
        (Default|UpdateExpiredAnim (Variables|DontEdit|GetHealthNPostureWB) false)))))

(event Custom|BindOnConsumeEnd
  (params (ConsumedMark :type WB%20Mark%20V%202%20Object%20Reference))
  (EventDispatchers|BindEventtoOnConsumeEnd ConsumedMark (delegate Custom|ResetMarks)))

(fn AddMark
  (CallFunction|MarkTimer)
  (if (and (< (Variables|DontEdit|GetMarks) (Variables|Edit|GetMaxMarks)) (not (CallFunction|IsEnoughMarks)))
    (Math|Integer|IncrementInt (Variables|DontEdit|GetMarks)
      (:%20%20
        (Default|AddMarkUI (Variables|DontEdit|GetHealthNPostureWB))
        (Variables|DontEdit|SetbIsMarked true)))))

(fn ConsumeMark
  (params (BaseDamage :type Float%20%28double-precision%29))
  (if (> (Variables|DontEdit|GetMarks) 0)
    (LocalVariables|SetDamage (CallFunction|CalculateDamage BaseDamage))
    (bind _output_get (LocalVariables|SetConsumedMarks (Variables|DontEdit|GetMarks)))
    (CallFunction|ResetMarks)
    (return (LocalVariables|GetDamage) _output_get)))

(fn CalculateDamage
  (params (BaseDamage :type Float%20%28double-precision%29))
  (bind _markdamagemultiplier (Variables|Edit|GetMarkDamageMultiplier))
  (for _index (range 0 (- (Variables|DontEdit|GetMarks) 1))
    (LocalVariables|SetTotalMultiplier (+ (LocalVariables|GetTotalMultiplier) (Utilities|Array|Get(acopy) _markdamagemultiplier (Math|Integer|Min(Integer) _index (Utilities|Array|LastIndex _markdamagemultiplier))))))
  (return (* BaseDamage (LocalVariables|GetTotalMultiplier))))

(fn IsEnoughMarks
  (bind _asbp_game_instance (Utilities|Casting|CastToBP_GameInstance (Game|GetGameInstance)))
  (return (>= (CallFunction|CalculateDamage (Default|GetMCBulletDamage _asbp_game_instance)) (Variables|/Game/Blueprint/Components/BPC_Health.BPC_Health_C|GetHealth (Variables|/Game/UI/Enemies/WB_HealthNPostureBar_v3.WB_HealthNPostureBar_v3_C|GetHealthComponent (Variables|DontEdit|GetHealthNPostureWB))))))

(fn PlayAddMarkSound
  (bind _markdamagemultiplier (Variables|Edit|GetMarkDamageMultiplier))
  (bind _returnvalue (Utilities|Array|Length _markdamagemultiplier))
  (bind _output_get (LocalVariables|SetSoundIndex (- (Variables|DontEdit|GetMarks) 1)))
  (if (>= _output_get _returnvalue)
    (bind _output_get_2 (LocalVariables|SetSoundIndex _returnvalue))
    (Math|Integer|DecrementInt _output_get_2
      (:%20%20
        _)))
  (Audio|PlaySoundatLocation (Utilities|Select :Index (LocalVariables|GetSoundIndex) :Option%200 (Variables|Audio|GetAdd1MarkSound) :Option%201 (Variables|Audio|GetAdd2MarkSound) :Option%202 (Variables|Audio|GetAdd3MarkSound)) (Transformation|GetActorLocation (Components|GetOwner)) "0, 0, 0" 1.0 1.0 0.0 0 0 0 0))

(fn PlayMarkExpireSound
  (Audio|PlaySoundatLocation (Variables|Audio|GetExpireMarkSound) (Transformation|GetActorLocation (Components|GetOwner)) "0, 0, 0" 1.0 1.0 0.0 0 0 0 0))