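; Health component that tracks an actor's health, clamped between zero and max, and handles its death.
; Reaching zero health ragdolls the owner's skeletal mesh, then branches on whether the owner implements BPI_MC.
; BPI_MC owners trigger game over on BP_MCController, lose input and capsule collision, then end the level.
; Other pawns detach from their controller and get an OnDeath call.
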(event Custom|RestartLevel
  (bind _asbp_mccontroller (Utilities|Casting|CastToBP_MCController (Game|GetPlayerController 0)))
  (Default|EndLevel _asbp_mccontroller))

(event EventBeginPlay
  (Variables|Default|SetHealth (Variables|Default|GetMaxHealth))
  (bind _asbp_mccontroller (Utilities|Casting|CastToBP_MCController (Game|GetPlayerController 0)))
  (Variables|Default|SetPlayerHUDRef (Variables|/Game/Blueprint/MC/BP_MCController.BP_MCController_C|GetPlayerHUD _asbp_mccontroller)))

(fn DecreaseHealth
  (params (Amount :type Float%20%28double-precision%29))
  (Variables|Default|SetHealth (Math|Float|Clamp(Float) (- (Variables|Default|GetHealth) Amount) 0.0 (Variables|Default|GetMaxHealth)))
  (if (<= (Variables|Default|GetHealth) 0.0)
    (CallFunction|Die)))

(fn IncreaseHealth
  (params (Amount :type Float%20%28double-precision%29))
  (Variables|Default|SetHealth (Math|Float|Clamp(Float) (+ Amount (Variables|Default|GetHealth)) 0.0 (Variables|Default|GetMaxHealth))))

(fn Die
  (bind _returnvalue (Components|GetOwner))
  (bind _returnvalue_2 (Components|GetOwner))
  (bind _returnvalue_3 (Actor|GetComponentbyClass _returnvalue "/Script/Engine.SkeletalMeshComponent"))
  (Collision|SetCollisionEnabled _returnvalue_3 "QueryAndPhysics")
  (Physics|SetSimulatePhysics _returnvalue_3 true)
  (if (Utilities|DoesObjectImplementInterface (Components|GetOwner) "/Game/Blueprint/MC/BPI_MC.BPI_MC_C")
    (Default|GameOver (.AsBP%20MCController (Utilities|Casting|CastToBP_MCController (Game|GetPlayerController 0))))
    (Input|DisableInput _returnvalue_2 0)
    (Collision|SetCollisionEnabled (Actor|GetComponentbyClass _returnvalue_2 "/Script/Engine.CapsuleComponent") "NoCollision")
    (CallFunction|RestartLevel)
    (else
      (bind _aspawn (Utilities|Casting|CastToPawn _returnvalue_2))
      (Class|Pawn|DetachfromControllerPendingDestroy _aspawn)
      (Default|CallOnDeath (Components|GetOwner)))))