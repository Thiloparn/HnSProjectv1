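; Player character's weapon that channels a projectile at the muzzle, then fires it, with fire cooldown and timed reload.
; ChannelBullet attaches a collisionless bullet, growing and recoloring it via timelines paced by the owner's charge time, with shake and particles when charged.
; Shoot detaches and launches it, then updates the HUD; CancelBullet destroys an unfired one.
; SubtractBullet's logic is disconnected, so shooting neither consumes ammo nor auto-reloads.
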(event Custom|Reload
  ;[1 1 1] Reload
  (if (not (Variables|Default|GetisReloading))
    (bind _asbp_mccharacter (Utilities|Casting|CastToBP_MCCharacter (Actor|GetParentActor)))
    (Default|PlayReloadAnimation _asbp_mccharacter)
    (Variables|Default|SetisReloading true)
    (bind _alpha (Timeline|TL_Reload PlayFromStart)
      (:Update
        (Variables|Default|SetElapsedReloadTime _alpha))
      (:Finished
        (Variables|Default|SetisReloading false)
        (Variables|Default|SetCurrentNumberOfBullets (Variables|Default|GetAmmoCapacity))
        (Default|UpdateBulletDisplay (Variables|Default|GetPlayerHUD))))))

(event Custom|Cooldown
  ;[1 1 1] Cooldown
  (Utilities|FlowControl|Delay (Variables|Default|GetFireRate))
  (Variables|Default|SetbIsInFireCooldown false))

(event Custom|ChannelBullet
  (bind _particlesystem_channeled (Variables|Default|GetParticleSystem_Channeled))
  ;[1 1 1] Channel Bullet
  (bind _returnvalue (Game|SpawnActorfromClass (Variables|Default|GetBulletType) (Transformation|GetWorldTransform (Variables|Default|GetSC_BulletSpawn)) "Undefined" "MultiplyWithRoot" self "EnemyBullet" 0))
  (bind _asbp_bullet_mc (Utilities|Casting|CastToBP_Bullet_MC _returnvalue))
  (bind _output_get (Variables|Default|SetBulletToShoot _asbp_bullet_mc))
  (Transformation|AttachComponentToComponent _output_get (Variables|Default|GetSC_BulletSpawn) "None" "SnapToTarget" "SnapToTarget" "SnapToTarget" true)
  (Collision|SetCollisionEnabled (Variables|/Game/Blueprint/Bullets/BP_Bullet.BP_Bullet_C|GetSphereCollision (Variables|Default|GetBulletToShoot)) "NoCollision")
  (Variables|Default|SetBulletToShootMaxScale (Transformation|GetActorScale3D (Variables|Default|GetBulletToShoot)))
  (Transformation|SetActorScale3D (Variables|Default|GetBulletToShoot) "0, 0, 0")
  (Utilities|FlowControl|Sequence
    (:then_0
      (bind _alpha (Timeline|TL_FormBullet PlayFromStart)
        (:Update
          (Utilities|IsValid (Variables|Default|GetBulletToShoot)
            (:Is%20Valid
              (Transformation|SetActorScale3D (Variables|Default|GetBulletToShoot) (Math|Vector|Lerp(Vector) "0, 0, 0" (Variables|Default|GetBulletToShootMaxScale) _alpha)))
            (:Is%20Not%20Valid
              (Timeline|TL_FormBullet Stop))))))
    (:then_1
      (bind _alpha_2 (Timeline|TL_ChangeColor PlayFromStart)
        (:Update
          (Utilities|IsValid (Variables|Default|GetBulletToShoot)
            (:Is%20Valid
              (bind _returnvalue_2 (Rendering|Material|CreateDynamicMaterialInstance (Variables|/Game/Blueprint/Bullets/BP_Bullet.BP_Bullet_C|GetStaticMesh (Variables|Default|GetBulletToShoot)) 0 "/Game/Materials/M_Bullet_MC.M_Bullet_MC" "None" :!class /Script/Engine.PrimitiveComponent))
              (Rendering|Material|SetVectorParameterValue _returnvalue_2 "Color" (Math|Color|Lerp(LinearColor) (Variables|Default|GetColorStartChannel) (Variables|Default|GetColor%20Finish%20Channel) _alpha_2) :!class /Script/Engine.MaterialInstanceDynamic))
            (:Is%20Not%20Valid
              (Timeline|TL_ChangeColor Stop))))
        (:Finished
          (Camera|PlayWorldCameraShake "/Game/Blueprint/CameraShakes/BP_BulletChannelledCameraShake.BP_BulletChannelledCameraShake_C" (Transformation|GetActorLocation (Game|GetPlayerCharacter 0)) 0.0 2e+03)
          (Components|Activation|Activate _particlesystem_channeled false)
          (Utilities|FlowControl|Delay 1.0)
          (Components|Activation|Deactivate _particlesystem_channeled))))))

(event Custom|ShootBullet
  (bind _bullettoshoot (Variables|Default|GetBulletToShoot))
  (bind _bullettoshoot_2 (Variables|Default|GetBulletToShoot))
  ;[1 1 1] ShootBullet
  (Utilities|IsValid _bullettoshoot_2
    (:Is%20Valid
      (Transformation|DetachFromActor _bullettoshoot_2 "KeepWorld" "KeepWorld" "KeepWorld")
      (Components|Activation|Activate (Variables|Default|GetParticleSystem_Muzzle) false)
      (Components|Activation|SetActive (Variables|/Game/Blueprint/Bullets/BP_Bullet.BP_Bullet_C|GetProjectileMovement (Variables|Default|GetBulletToShoot)) true false)
      (Variables|/Script/Engine.MovementComponent|SetVelocity (Variables|/Game/Blueprint/Bullets/BP_Bullet.BP_Bullet_C|GetProjectileMovement _bullettoshoot) (* (Math|Vector|Normalize (Math|Vector|GetForwardVector (Variables|Default|GetSC_BulletSpawn))) (Variables|/Game/Blueprint/Bullets/BP_Bullet.BP_Bullet_C|GetBulletSpeed _bullettoshoot)))
      (Collision|SetCollisionEnabled (Variables|/Game/Blueprint/Bullets/BP_Bullet.BP_Bullet_C|GetSphereCollision (Variables|Default|GetBulletToShoot)) "QueryAndPhysics"))))

(event Custom|CancelBullet
  ;[1 1 1] Cancel Bullet
  (Utilities|IsValid (Variables|Default|GetBulletToShoot)
    (:Is%20Valid
      (if (== (Transformation|GetAttachParent (Variables|/Game/Blueprint/Bullets/BP_Bullet.BP_Bullet_C|GetSphereCollision (Variables|Default|GetBulletToShoot))) (Variables|Default|GetSC_BulletSpawn))
        (Actor|DestroyActor (Variables|Default|GetBulletToShoot))
        (Variables|Default|SetBulletToShoot 0)))))

(event EventBeginPlay
  (Rendering|SetCastShadow (Variables|Default|GetArrowWidget) false)
  (Variables|Default|SetBulletSpawnTrasnform (Transformation|GetRelativeTransform (Variables|Default|GetSC_BulletSpawn)))
  (Variables|Default|SetCurrentNumberOfBullets (Variables|Default|GetAmmoCapacity))
  (Components|Timeline|SetPlayRate (Variables|Default|GetTL_Reload) (/ 1.0 (Variables|Default|GetReloadTime)))
  (bind _shootchargetime (Class|BPIMC|GetShootChargeTime(Message) (Actor|GetParentActor)))
  (Components|Timeline|SetPlayRate (Variables|Default|GetTL_FormBullet) (/ 1.0 _shootchargetime))
  (bind _asbp_mccontroller (Utilities|Casting|CastToBP_MCController (Game|GetPlayerController 0)))
  (Variables|Default|SetPlayerHUD (Variables|/Game/Blueprint/MC/BP_MCController.BP_MCController_C|GetPlayerHUD _asbp_mccontroller)))

(fn ConstructionScript
  (Variables|Default|SetColorStartChannel "(R=1.000000,G=0.913099,B=0.234551,A=1.000000)")
  (Variables|Default|SetColor%20Finish%20Channel "(R=1.000000,G=0.000000,B=0.597202,A=1.000000)"))

(fn SubtractBullet)

(fn Shoot
  (if (not (Variables|Default|GetisReloading))
    (if (not (Variables|Default|GetbIsInFireCooldown))
      (Variables|Default|SetbIsInFireCooldown true)
      (CallFunction|ShootBullet)
      (CallFunction|ResetBulletSpawn)
      (CallFunction|SubtractBullet)
      (Default|UpdateBulletDisplay (Variables|Default|GetPlayerHUD))
      (CallFunction|Cooldown)
      (return true)
      (else
        _)))
  (return false))

(fn ResetBulletSpawn
  (Transformation|SetRelativeTransform (Variables|Default|GetSC_BulletSpawn) (Variables|Default|GetBulletSpawnTrasnform) false false))

(fn GetIsReloading
  (return (Variables|Default|GetisReloading)))